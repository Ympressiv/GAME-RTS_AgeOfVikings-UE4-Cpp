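; Player controller that links the level's hex grid to the Graph A* navmesh and handles grid clicks.
; On BeginPlay it looks up both actors and prints if either is missing, but sets HexGrid to None rather than the found grid before passing it to the navmesh.
; SecondaryAction passes the location under the cursor to the grid's SnapToGrid when HexGrid is valid, discarding any result.
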(event EventBeginPlay
  (bind _returnvalue (Actor|GetActorOfClass "/Game/Blueprints/HexagonalGrid/BP_HexGrid.BP_HexGrid_C"))
  (Utilities|IsValid _returnvalue
    (:Is%20Valid
      (Variables|Default|SetHexGrid 0)
      (bind _returnvalue_2 (Actor|GetActorOfClass "/Script/RTS_AoV.GraphAStarNavMesh"))
      (Utilities|IsValid _returnvalue_2 ; Just to be sure.
        (:Is%20Valid
          (bind _output_get (Variables|Default|SetGASNavMesh _returnvalue_2))
          (Class|GraphAStarNavMesh|SetHexGrid _output_get (Variables|Default|GetHexGrid)))
        (:Is%20Not%20Valid
          (Development|PrintString "GraphAStarNavMesh not present or invalid,  
maybe try to rebuild it?" true true "(R=1.000000,G=0.000000,B=0.000000,A=1.000000)" 5.0))))
    (:Is%20Not%20Valid
      (Development|PrintString "No HexGrid available, please drop one in the level!" false true "(R=1.000000,G=0.000000,B=0.000000,A=1.000000)" 5.0))))

(event Input|ActionEvents|InputActionSecondaryAction
  (params (Key :type Key%20Structure :default "None"))
  (bind _hexgrid (Variables|Default|GetHexGrid))
  (:Pressed
    (Utilities|IsValid _hexgrid
      (:Is%20Valid
        (Class|HexGrid|SnaptoGrid _hexgrid (.Location (Collision|BreakHitResult (.HitResult (Game|Player|GetHitResultUnderCursorbyChannel "TraceTypeQuery1" true)))))))))

(fn ConstructionScript)