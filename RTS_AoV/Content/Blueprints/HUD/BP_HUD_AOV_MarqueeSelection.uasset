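; HUD that draws a click-and-drag marquee rectangle on screen, apparently for RTS-style unit selection.
; OnInputStart anchors the box at the mouse position only when SelectedUnits is empty, OnInputHold moves the opposite corner, and OnInputRelease stops drawing.
; While drawing, DrawHUD renders both corner points and a translucent blue rectangle between them.
; No unit selection happens in this graph; SelectedUnits is only read.
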(event Custom|DrawMarquee
  (bind _clickedlocation (Variables|MarqueeVariables|GetClickedLocation))
  (bind _holdinglocation (Variables|Default|GetHoldingLocation))
  (bind _clickedlocation_2 (Variables|MarqueeVariables|GetClickedLocation))
  (bind _holdinglocation_2 (Variables|Default|GetHoldingLocation))
  (bind (_x _y) (Math|Vector2D|BreakVector2D _holdinglocation_2))
  (bind (_x_2 _y_2) (Math|Vector2D|BreakVector2D _clickedlocation_2))
  (bind _returnvalue (- _holdinglocation _clickedlocation_2))
  (bind (_x_3 _y_3) (Math|Vector2D|BreakVector2D _clickedlocation))
  (bind (_x_4 _y_4) (Math|Vector2D|BreakVector2D _returnvalue))
  (HUD|DrawRect "(R=0,G=0,B=0,A=1)" _x_3 _y_3 0.0 0.0)
  (HUD|DrawRect "(R=0.000000,G=0.000000,B=0.026000,A=1.000000)" _x _y 0.0 0.0)
  (HUD|DrawRect "(R=0.000000,G=0.213754,B=1.000000,A=0.608000)" _x_2 _y_2 _x_4 _y_4))

(event EventBeginPlay
  (Variables|Refrences|SetBP%20AOV%20Player%20Controller (.AsBP%20AOV%20Player%20Controller (Utilities|Casting|CastToBP_AOV_PlayerController (Game|GetPlayerController 0)))))

(event EventOnInputStart
  (bind _bp_aov_player_controller (Variables|Refrences|GetBP%20AOV%20Player%20Controller))
  (bind (_locationx _locationy) (Game|Player|GetMousePosition _bp_aov_player_controller))
  (if (not (>= (Utilities|Array|LastIndex (Variables|Units|GetSelectedUnits)) 0))
    (bind _output_get (Variables|MarqueeVariables|SetClickedLocation (Math|Vector2D|MakeVector2D _locationx _locationy)))
    (Variables|Default|SetHoldingLocation _output_get)
    (Variables|Bool|SetIsDrawing true)))

(event EventOnInputRelease
  (params (HoldTime :type Float%20%28single-precision%29))
  (Variables|Bool|SetIsDrawing false))

(event EventDrawHUD
  (params (SizeX :type Integer) (SizeY :type Integer))
  (if (Variables|Bool|GetIsDrawing)
    (Utilities|FlowControl|Sequence
      (:then_0
        (CallFunction|DrawMarquee)))))

(event EventOnInputHold
  (bind _bp_aov_player_controller (Variables|Refrences|GetBP%20AOV%20Player%20Controller))
  (bind (_locationx _locationy) (Game|Player|GetMousePosition _bp_aov_player_controller))
  (Variables|Default|SetHoldingLocation (Math|Vector2D|MakeVector2D _locationx _locationy)))

(fn ConstructionScript)