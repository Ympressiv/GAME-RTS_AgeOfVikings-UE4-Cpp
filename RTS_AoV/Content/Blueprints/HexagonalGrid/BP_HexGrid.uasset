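; Hex grid actor that generates a tile map in cube coordinates with random costs, blocking tiles and a portal.
; The Construction Script calls CreateGrid, using its per-coordinate delegate to build tiles as two instanced meshes, with regular tile height scaled by cost.
; One edge coordinate receives the child-actor portal instead of a mesh, which BeginPlay initializes.
; A looping timer redraws coordinate and cost labels, toggled by H and C.
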(event Custom|DebugDraws
  ;[1 0.2865 0.2865] Draw tiles Cube Coordinates and/or tiles cost (debug).
  (if (or (Variables|Default|GetDebugCoords) (Variables|Default|GetDebugCost))
    (for _array_element (Variables|Default|GetGridTiles)
      (if (Variables|Default|GetDebugCoords)
        (CallFunction|DrawDebugCoords (.CubeCoord (Utilities|Struct|BreakHexTile _array_element)) (.WorldPosition (Utilities|Struct|BreakHexTile _array_element)) (Variables|Default|GetDebugTimerDuration)))
      (if (and (Variables|Default|GetDebugCost) (not (.bIsBlocking (Utilities|Struct|BreakHexTile _array_element))))
        (CallFunction|DrawDebugCost (.WorldPosition (Utilities|Struct|BreakHexTile _array_element)) (.Cost (Utilities|Struct|BreakHexTile _array_element)) (Variables|Default|GetDebugTimerDuration))))))

(event Custom|OnTimerTick
  ;[1 0.224 0.224] Start the timer for debug draws
  (CallFunction|DebugDraws))

(event EventBeginPlay
  ;[1 1 1] Init the BP_Portal actor
  (bind _asbp_portal (Utilities|Casting|CastToBP_Portal (Variables|/Script/Engine.ChildActorComponent|GetChildActor (Variables|Default|GetPortal))))
  (Default|Init _asbp_portal (Variables|Default|GetPortalText) (Variables|Default|GetPortalCounter) (Variables|Default|GetPortalMapToOpen))
  ;[1 0.224 0.224] Start the timer for debug draws
  (Utilities|Time|SetTimerbyEvent (delegate Custom|OnTimerTick) (Variables|Default|GetDebugTimerDuration) true)
  (CallFunction|DebugDraws))

(event Input|KeyboardEvents|C
  (params (Key :type Key%20Structure :default "None"))
  ;[1 0.2865 0.2865] Draw tiles Cube Coordinates and/or tiles cost (debug).
  ;;[1 1 1] Debug Tile Cost hotkey
  (:Pressed
    (bind _isa (Utilities|FlowControl|FlipFlop)
      (:A
        _)
      (:B
        _))
    (Variables|Default|SetDebugCost _isa)))

(event Input|KeyboardEvents|H
  (params (Key :type Key%20Structure :default "None"))
  ;[1 0.2865 0.2865] Draw tiles Cube Coordinates and/or tiles cost (debug).
  ;;[1 1 1] Debug Cube Coordinates hotkey
  (:Pressed
    (bind _isa (Utilities|FlowControl|FlipFlop)
      (:A
        _)
      (:B
        _))
    (Variables|Default|SetDebugCoords _isa)))

(fn ConstructionScript
  ;[1 1 1] Clean up the internal grid arrays
  (Utilities|Array|Clear (Variables|Default|GetGridTiles))
  (Utilities|Array|Clear (Variables|Default|GetGridCoordinates))
  ;[1 1 1] Clean up our Instanced Static Mesh Components.
  (Components|InstancedStaticMesh|ClearInstances (Variables|Default|GetISM_RegularTile))
  ;[0.3571 0.7109 1] Set the current actor location as our origin.
  (bind _structout (Utilities|Struct|SetmembersinHTileLayout (Variables|Default|GetTlayout) (Transformation|GetActorLocation)))
  ;[0.3571 0.7109 1] Here we ceate the "logical part" of the grid, this function just compute and store in an array the coordinates in Cube format.
  ;
  ; This function has an optional delegate, this delegate is fired at every new created coordinate.
  ;
  ; In our example we use it to create the "concrete part" of our grid, the tiles.
  (Class|HexGrid|CreateGrid _structout (Variables|Default|GetGridRadius) (EventDispatchers|CreateEvent :!event AddTile)))

(fn AddTile
  (params (TileLayout :type H%20Tile%20Layout%20Structure%20%28by%20ref%29) (Coord :type H%20Cube%20Coord%20Structure%20%28by%20ref%29))
  ;[1 1 1] Store the TileLayout in a local variable and convert the Cube Coordinate to World Space coordinate.
  (LocalVariables|SetTileLayout_Local TileLayout)
  (bind _returnvalue (Class|HexGrid|HextoWorld Coord))
  (bind _output_get (LocalVariables|SetTileLocation_Local _returnvalue))
  ;[1 1 1] Setup the transform for our portal, we want only one in our map so Done will be true only once, look at the SetPortalLocation implementation.
  (bind _done (CallFunction|SetPortalLocation Coord (CallFunction|CalculateTransform (LocalVariables|GetTileLayout_Local) _output_get 1.0 "0, 0, 0" "0,-30.000000, 0")))
  (if _done
    ;[1 1 1] If we moved the portal in the desired location set the tile in his position as non blocking and with cost 1.
    ;
    ; Also we skip the addition of a new element to ISM component.
    (LocalVariables|SetTileCost_Local 1.0)
    (LocalVariables|SetIsBlocking_Local false)
    (Utilities|Array|Add (Variables|Default|GetGridTiles) (Utilities|Struct|MakeHexTile Coord (LocalVariables|GetTileLocation_Local) (LocalVariables|GetTileCost_Local) (LocalVariables|GetIsBlocking_Local)))
    (return)
    (else
      ;[1 1 1] Set a random value to Cost and IsBlocking and add the tile to the array.
      (LocalVariables|SetTileCost_Local (Math|Random|RandomFloatinRange (Variables|Default|GetMinCost) (Variables|Default|GetMaxCost)))
      (LocalVariables|SetIsBlocking_Local (Math|Random|RandomBoolwithWeight (Variables|Default|GetBlockWeight)))
      (Utilities|Array|Add (Variables|Default|GetGridTiles) (Utilities|Struct|MakeHexTile Coord (LocalVariables|GetTileLocation_Local) (LocalVariables|GetTileCost_Local) (LocalVariables|GetIsBlocking_Local)))
      (if (LocalVariables|GetIsBlocking_Local)
        ;[1 1 1] If is a blocking tile set add it to the dedicated ISM component and we scale the Z axis by a fixed value.
        (LocalVariables|SetTileScaleZ_Local (Variables|Default|GetBlockHeight))
        (Class|InstancedStaticMeshComponent|AddInstanceWorldSpace (Variables|Default|GetISM_BlockingTile) (CallFunction|CalculateTransform (LocalVariables|GetTileLayout_Local) (LocalVariables|GetTileLocation_Local) (LocalVariables|GetTileScaleZ_Local) "0, 0, 0" "0,30.000000, 0"))
        (else
          ;[1 1 1] If is a normal tile (non blocking) we scale up Z by two time the cost of the tile.
          (LocalVariables|SetTileScaleZ_Local (* (LocalVariables|GetTileCost_Local) 2.0))
          (Class|InstancedStaticMeshComponent|AddInstanceWorldSpace (Variables|Default|GetISM_RegularTile) (CallFunction|CalculateTransform (LocalVariables|GetTileLayout_Local) (LocalVariables|GetTileLocation_Local) (LocalVariables|GetTileScaleZ_Local) "0, 0, 0" "0,30.000000, 0"))))
      (return))))

(fn DrawDebugCoords
  (params (H :type H%20Cube%20Coord%20Structure%20%28by%20ref%29) (V :type Vector) (Duration :type Float%20%28single-precision%29))
  (bind _qrs (Utilities|Struct|BreakHCubeCoord H))
  (bind _returnvalue (+ V "-50.000000, 0, 0"))
  (bind _returnvalue_2 (+ V "50.000000,-50.000000, 0"))
  (bind _returnvalue_3 (+ V "50.000000,50.000000,0.000000"))
  (LocalVariables|SetDuration_Local Duration)
  (bind _returnvalue_4 (Class|HexGrid|HexEqual H (Utilities|Struct|MakeHCubeCoord "(X=0,Y=0,Z=0)")))
  (if _returnvalue_4
    ;[1 1 1] At (0, 0, 0)
    (Rendering|Debug|DrawDebugString _returnvalue_2 "X" 0 "(R=0.000000,G=1.000000,B=0.000000,A=1.000000)" (LocalVariables|GetDuration_Local))
    (Rendering|Debug|DrawDebugString _returnvalue_3 "Y" 0 "(R=0.000000,G=0.000000,B=1.000000,A=1.000000)" (LocalVariables|GetDuration_Local))
    (Rendering|Debug|DrawDebugString _returnvalue "Z" 0 "(R=1.000000,G=0.000000,B=0.000000,A=1.000000)" (LocalVariables|GetDuration_Local))
    (else
      (Rendering|Debug|DrawDebugString _returnvalue_2 (Utilities|String|ToString(Integer) (.x _qrs)) 0 "(R=0.000000,G=1.000000,B=0.000000,A=1.000000)" (LocalVariables|GetDuration_Local))
      (Rendering|Debug|DrawDebugString _returnvalue_3 (Utilities|String|ToString(Integer) (.y _qrs)) 0 "(R=0.000000,G=0.000000,B=1.000000,A=1.000000)" (LocalVariables|GetDuration_Local))
      (Rendering|Debug|DrawDebugString _returnvalue (Utilities|String|ToString(Integer) (.z _qrs)) 0 "(R=1.000000,G=0.000000,B=0.007957,A=1.000000)" (LocalVariables|GetDuration_Local)))))

(fn DrawDebugCost
  (params (V :type Vector) (C :type Float%20%28single-precision%29) (Duration :type Float%20%28single-precision%29))
  (Rendering|Debug|DrawDebugString V (Utilities|String|ToString(Text) (Utilities|Text|ToText(Float) C "HalfToEven" false true 1 324 0 1)) 0 "(R=1.000000,G=1.000000,B=1.000000,A=1.000000)" Duration))

(fn SetPortalLocation
  (params (HCubeCoord :type H%20Cube%20Coord%20Structure%20%28by%20ref%29) (SpawnTransform :type Transform))
  (bind _qrs (Utilities|Struct|BreakHCubeCoord HCubeCoord))
  (bind (_x _y _z) (Utilities|Struct|BreakIntVector _qrs))
  (if (and (== _x 0) (== _z (Variables|Default|GetGridRadius)))
    (Transformation|SetWorldTransform (Variables|Default|GetPortal) SpawnTransform false false)
    (return true)
    (else
      ;[1 1 1] Skip if we are not on the right coordinate.
      (return false))))

(fn CalculateTransform
  (params (HTileLayout :type H%20Tile%20Layout%20Structure%20%28by%20ref%29) (TileLocation :type Vector) (TileScaleZ :type Float%20%28single-precision%29) (FLAT :type Rotator) (POINTY :type Rotator))
  (return (Math|Transform|MakeTransform TileLocation (Utilities|Select :Index (Utilities|Struct|BreakHTileLayout HTileLayout) :FLAT FLAT :POINTY POINTY :NONE "0, 0, 0") (Math|Vector|MakeVector 1.0 1.0 TileScaleZ))))